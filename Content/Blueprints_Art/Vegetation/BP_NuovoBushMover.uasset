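; Component that makes its owning BP_Bush_Base rustle when the ThirdPersonCharacter enters it.
; EnterBush plays a bush sound at the owner's location and fakes a shake by rotating the CespugliCespuglio1 component back and forth in short delayed steps, with no timeline.
; An AlreadyMoved flag blocks retriggering until ExitBush clears it after a one-second delay.
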(event Custom|EnterBush
  (params (Player :type Object%20Object%20Reference))
  (bind _returnvalue (Components|GetOwner))
  (bind _asbp_bush_base (Utilities|Casting|CastToBP_Bush_Base _returnvalue))
  (bind _cespugli_cespuglio_1 (Variables|/Game/Blueprints_Art/Vegetation/BP_Bush_Base.BP_Bush_Base_C|GetCespugli_Cespuglio_1 _asbp_bush_base))
  (if (not (Variables|Default|GetAlready%20Moved))
    (Utilities|Casting|CastToThirdPersonCharacter Player)
    (Variables|Default|SetAlready%20Moved true)
    (Audio|PlaySoundatLocation "/Game/Audio/SFXs/ENV_Sounds/Bush_SFX_Cue.Bush_SFX_Cue" (Transformation|GetActorLocation (Components|GetOwner)) "0, 0, 0" 1.0 1.0 0.0 0 0 0)
    (Transformation|AddWorldRotation _cespugli_cespuglio_1 "0, 0,-4.000000" false false)
    (Utilities|FlowControl|Delay 0.05)
    (Transformation|AddWorldRotation _cespugli_cespuglio_1 "0, 0,8.000000" false false)
    (Utilities|FlowControl|Delay 0.05)
    (Transformation|AddWorldRotation _cespugli_cespuglio_1 "0, 0,-4.000000" false false)))

(event Custom|ExitBush
  (params (Player :type Object%20Object%20Reference))
  (Utilities|Casting|CastToThirdPersonCharacter Player)
  (Utilities|FlowControl|Delay 1.0)
  (Variables|Default|SetAlready%20Moved false))
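; Photo album Blueprint that serves as a diary, showing unlocked text entries as material changes on the book mesh.
; DisplayText01–03 set unlock flags on the SaveVariables game instance and fill the first free OccupiedSlots entry with a red material.
; LoadDiary clears the slots and replays unlocked entries in numeric order, regardless of unlock order.
; On load, the third entry always paints material element 0 instead of its slot index.
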(event Custom|LoadDiary
  (bind _occupiedslots (Variables|Default|GetOccupiedSlots))
  (for (_ _array_index) _occupiedslots
    (Utilities|Array|SetArrayElem _occupiedslots _array_index false))
  (if (Variables|/Game/Blueprints_Design/SaveVariables.SaveVariables_C|GetDiaryText01_Unlocked (.AsSave%20Variables (Utilities|Casting|CastToSaveVariables (Game|GetGameInstance))))
    (Development|PrintString "Text1 Loaded")
    (bind (_array_element _array_index_2) (Utilities|Array|ForEachLoopwithBreak (Variables|Default|GetOccupiedSlots) :!label _label)
      (:LoopBody
        (if (Math|Boolean|Equal(Boolean) _array_element false)
          (Rendering|Material|SetMaterial (Variables|Default|GetSK_PhotoBook01) _array_index_2 "/AnimationSharing/AnimSharingRed.AnimSharingRed")
          (Utilities|Array|SetArrayElem (Variables|Default|GetOccupiedSlots) _array_index_2 true)
          (goto _label Break)))
      (:Completed
        (if (Variables|/Game/Blueprints_Design/SaveVariables.SaveVariables_C|GetDiaryText02_Unlocked (.AsSave%20Variables (Utilities|Casting|CastToSaveVariables (Game|GetGameInstance)))) :!label _label_2
          (Development|PrintString "Text2 Loaded")
          (bind (_array_element_2 _array_index_3) (Utilities|Array|ForEachLoopwithBreak (Variables|Default|GetOccupiedSlots) :!label _label_3)
            (:LoopBody
              (if (Math|Boolean|Equal(Boolean) _array_element_2 false)
                (Rendering|Material|SetMaterial (Variables|Default|GetSK_PhotoBook01) _array_index_3 "/AnimationSharing/AnimSharingRed.AnimSharingRed")
                (Utilities|Array|SetArrayElem (Variables|Default|GetOccupiedSlots) _array_index_3 true)
                (goto _label_3 Break)))
            (:Completed
              (if (Variables|/Game/Blueprints_Design/SaveVariables.SaveVariables_C|GetDiaryText03_Unlocked (.AsSave%20Variables (Utilities|Casting|CastToSaveVariables (Game|GetGameInstance)))) :!label _label_4
                (Development|PrintString "Text3 Loaded")
                (bind (_array_element_3 _array_index_4) (Utilities|Array|ForEachLoopwithBreak (Variables|Default|GetOccupiedSlots) :!label _label_5)
                  (:LoopBody
                    (if (Math|Boolean|Equal(Boolean) _array_element_3 false)
                      (Rendering|Material|SetMaterial (Variables|Default|GetSK_PhotoBook01) 0 "/AnimationSharing/AnimSharingRed.AnimSharingRed")
                      (Utilities|Array|SetArrayElem (Variables|Default|GetOccupiedSlots) _array_index_4 true)
                      (goto _label_5 Break)))
                  (:Completed
                    (Development|PrintString "DiaryLoaded" :!label _label_6)))
                (else
                  (goto _label_6)))))
          (else
            (goto _label_4)))))
    (else
      (goto _label_2))))

(event Custom|DisplayText01
  (Variables|/Game/Blueprints_Design/SaveVariables.SaveVariables_C|SetDiaryText01_Unlocked (.AsSave%20Variables (Utilities|Casting|CastToSaveVariables (Game|GetGameInstance))) true)
  (bind (_array_element _array_index) (Utilities|Array|ForEachLoopwithBreak (Variables|Default|GetOccupiedSlots) :!label _label)
    (:LoopBody
      (if (Math|Boolean|Equal(Boolean) _array_element false)
        (Rendering|Material|SetMaterial (Variables|Default|GetSK_PhotoBook01) _array_index "/AnimationSharing/AnimSharingRed.AnimSharingRed")
        (Utilities|Array|SetArrayElem (Variables|Default|GetOccupiedSlots) _array_index true)
        (goto _label Break)))))

(event Custom|DisplayText03
  (Variables|/Game/Blueprints_Design/SaveVariables.SaveVariables_C|SetDiaryText03_Unlocked (.AsSave%20Variables (Utilities|Casting|CastToSaveVariables (Game|GetGameInstance))) true)
  (bind (_array_element _array_index) (Utilities|Array|ForEachLoopwithBreak (Variables|Default|GetOccupiedSlots) :!label _label)
    (:LoopBody
      (if (Math|Boolean|Equal(Boolean) _array_element false)
        (Rendering|Material|SetMaterial (Variables|Default|GetSK_PhotoBook01) _array_index "/AnimationSharing/AnimSharingRed.AnimSharingRed")
        (Utilities|Array|SetArrayElem (Variables|Default|GetOccupiedSlots) _array_index true)
        (goto _label Break)))))

(event Custom|DisplayText02
  (Variables|/Game/Blueprints_Design/SaveVariables.SaveVariables_C|SetDiaryText02_Unlocked (.AsSave%20Variables (Utilities|Casting|CastToSaveVariables (Game|GetGameInstance))) true)
  (bind (_array_element _array_index) (Utilities|Array|ForEachLoopwithBreak (Variables|Default|GetOccupiedSlots) :!label _label)
    (:LoopBody
      (if (Math|Boolean|Equal(Boolean) _array_element false)
        (Rendering|Material|SetMaterial (Variables|Default|GetSK_PhotoBook01) _array_index "/AnimationSharing/AnimSharingRed.AnimSharingRed")
        (Utilities|Array|SetArrayElem (Variables|Default|GetOccupiedSlots) _array_index true)
        (goto _label Break)))))

(fn ConstructionScript)